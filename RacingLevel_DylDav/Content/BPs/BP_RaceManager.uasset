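; BP_RaceManager is a race manager Blueprint that runs the start countdown and holds cars until GO.
; On BeginPlay it shows a WDG_321go countdown widget and disables movement on every car in Cars2, re-enabling it after a fixed delay.
; It also writes a newly created LapTimes save to an unnamed slot before the countdown and loads that slot again after the cars are released.
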(event EventBeginPlay
  (bind _returnvalue (SaveGame|CreateSaveGameObject "/Script/Engine.SaveGame"))
  (Variables|Default|SetLapTimes (Variables|Default|GetLapTimes))
  (SaveGame|SaveGametoSlot _returnvalue)
  (bind _returnvalue_2 (UserInterface|CreateWidget "/Game/BPs/WDG_321go.WDG_321go_C"))
  (Default|321 _returnvalue_2 3 "GO!")
  (UserInterface|Viewport|AddtoViewport _returnvalue_2 0)
  (CallFunction|ToggleCarsMovement false)
  (Utilities|FlowControl|Delay 8.0)
  (CallFunction|ToggleCarsMovement true)
  (SaveGame|LoadGamefromSlot)
  (Variables|Default|SetLapTimes (Variables|Default|GetLapTimes)))

(event Collision|EventActorBeginOverlap
  (params (OtherActor :type Actor%20Object%20Reference)))

(event EventTick
  (params (DeltaSeconds :type Float%20%28single-precision%29)))

(fn ConstructionScript)

(fn ToggleCarsMovement
  (params (MovementEnabled :type Boolean))
  (for _array_element (Variables|Default|GetCars2)
    (Variables|/Game/VehicleTemplate/Blueprints/VehicleAdvPawn.VehicleAdvPawn_C|SetMovementEnabled _array_element MovementEnabled)))