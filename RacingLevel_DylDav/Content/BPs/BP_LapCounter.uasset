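; BP_LapCounter is a trigger actor that counts the vehicle's laps and ends the race with a win.
; An IsFirstTime flag absorbs an initial crossing; later overlaps pass a DoOnce that increments Laps and updates the pawn's lap UI.
; After a short delay it plays lap sounds and resets the DoOnce, or at four laps shows the win widget, pauses and plays victory music.
; The Laptime overlap only casts.
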(event OnComponentBeginOverlap(Trigger)
  (params (OverlappedComponent :type Primitive%20Component%20Object%20Reference) (OtherActor :type Actor%20Object%20Reference) (OtherComp :type Primitive%20Component%20Object%20Reference) (OtherBodyIndex :type Integer) (bFromSweep :type Boolean) (SweepResult :type Hit%20Result%20Structure%20%28by%20ref%29))
  (bind _asvehicle_adv_pawn (Utilities|Casting|CastToVehicleAdvPawn OtherActor))
  (if (Variables|Default|GetisFirstTime)
    (Variables|Default|SetisFirstTime true)
    (Utilities|FlowControl|Delay 0.5)
    (Variables|Default|SetisFirstTime false)
    (else
      (Utilities|FlowControl|DoOnce false :!label _label
        (:Completed
          (Math|Integer|IncrementInt (Variables|Default|GetLaps)
            (:%20%20
              (Rendering|Components|TextRender|SetText (Variables|/Game/BPs/WP_LapCounter.WP_LapCounter_C|GetLapText (Variables|/Game/VehicleTemplate/Blueprints/VehicleAdvPawn.VehicleAdvPawn_C|GetLapCounterUI _asvehicle_adv_pawn)) (Utilities|Text|FormatText "Lap {Lap Number}" (Variables|Default|GetLaps)))
              (Utilities|FlowControl|Delay 0.7)
              (if (>= (Variables|Default|GetLaps) 4)
                (Input|SetInputModeUIOnly (Game|GetPlayerController 0) 0 "DoNotLock" true)
                (bind _returnvalue (UserInterface|CreateWidget "/Game/BPs/WP_Youwin.WP_Youwin_C"))
                (UserInterface|Viewport|AddtoViewport _returnvalue 0)
                (Game|SetGamePaused true)
                (Audio|PlaySound2D "/Game/BPs/Gaming_Themed__Royalty-Free__Music：_BoxCat_Games_-_＂Victory＂.Gaming_Themed__Royalty-Free__Music：_BoxCat_Games_-_＂Victory＂" 1.0 1.0 0.0 0 0)
                (elif (>= (Variables|Default|GetLaps) 3)
                  (Audio|PlaySound2D "/Game/BPs/1lap_01.1lap_01" 1.0 1.0 0.0 0 0)
                  (goto _label Reset)
                  (elif (>= (Variables|Default|GetLaps) 2)
                    (Audio|PlaySound2D "/Game/BPs/2lap_01.2lap_01" 1.0 1.0 0.0 0 0)
                    (goto _label Reset)
                    (else
                      (goto _label Reset))))))))))))

(event OnComponentEndOverlap(Trigger)
  (params (OverlappedComponent :type Primitive%20Component%20Object%20Reference) (OtherActor :type Actor%20Object%20Reference) (OtherComp :type Primitive%20Component%20Object%20Reference) (OtherBodyIndex :type Integer)))

(event OnComponentBeginOverlap(laptime)
  (params (OverlappedComponent :type Primitive%20Component%20Object%20Reference) (OtherActor :type Actor%20Object%20Reference) (OtherComp :type Primitive%20Component%20Object%20Reference) (OtherBodyIndex :type Integer) (bFromSweep :type Boolean) (SweepResult :type Hit%20Result%20Structure%20%28by%20ref%29))
  (Utilities|Casting|CastToVehicleAdvPawn OtherActor))

(event EventBeginPlay)

(event Collision|EventActorBeginOverlap
  (params (OtherActor :type Actor%20Object%20Reference)))

(event EventTick
  (params (DeltaSeconds :type Float%20%28single-precision%29)))

(fn ConstructionScript)